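; BP_OSC runs a local OSC server that lets external messages switch levels and teleport the player between markers.
; It handles addresses containing "/map", reading the level name before the dot and a marker ID after it.
; If that level is current, the player moves just above the matching BP_markerTeleport and takes its rotation as control rotation.
; Otherwise it only opens the named level, without applying the marker.
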(event `self.ReceiveBeginPlay`
  (bind _returnvalue (`OSCManager.CreateOSCServer` "127.0.0.1" 1337 false true "" null))
  (bind _output_get (set `self.OSC Server` _returnvalue))
  (add `OSCServer.OnOscMessageReceived` _output_get (`|CreateDelegate` :!event `OSC Message Recieved`)))

(event `OSC Message Recieved`
  (params (Message :type "OSCMessage Structure (by ref)") (IPAddress :type String) (Port :type Integer))
  (bind _returnvalue (`OSCManager.GetOSCMessageAddress` Message))
  (bind _returnvalue_2 (`OSCManager.GetOSCAddressFullPath` _returnvalue))
  (if (`KismetStringLibrary.Contains` _returnvalue_2 "/map")
    (bind _returnvalue_3 (`GameplayStatics.GetCurrentLevelName` true))
    (bind (_lefts _rights) (`KismetStringLibrary.Split` _returnvalue_2 "."))
    (if (`KismetStringLibrary.EqualEqual_StrStr` (`KismetStringLibrary.Concat_StrStr` "/" _returnvalue_3) _lefts)
      (bind _outactors (`GameplayStatics.GetAllActorsOfClass` "/Game/FajarRoshn/Blueprints/BP_markerTeleport.BP_markerTeleport_C"))
      (for _array_element _outactors
        (if (== (`/Game/FajarRoshn/Blueprints/BP_markerTeleport.markerID` _array_element) (`KismetStringLibrary.Conv_StringToInt` _rights))
          (bind (_returnvalue_x _returnvalue_y _returnvalue_z) (`KismetMathLibrary.BreakVector` (`self.K2_GetActorLocation` _array_element)))
          (`self.K2_SetActorLocation` (`GameplayStatics.GetPlayerCharacter` 0) (`KismetMathLibrary.MakeVector` _returnvalue_x _returnvalue_y (+ _returnvalue_z 100.0)) false false)
          (`Controller.SetControlRotation` (`GameplayStatics.GetPlayerController` 0) (`self.K2_GetActorRotation` _array_element))))
      (else
        (`GameplayStatics.OpenLevel` (`KismetStringLibrary.Conv_StringToName` (`KismetStringLibrary.RightChop` _lefts 1)))))))

(fn `UserConstructionScript`)