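; House Blueprint for the vd4_dp4 variant, configured entirely in the construction script with no active event logic.
; UsePlant toggles visibility of four HISM components and makes them Static when shown, Movable when hidden.
; Two text renders display Type, with TextRender1 re-rotated when any actor scale axis is negative, as when mirrored.
; Direct static mesh children of SharedRoot take their mobility from PlantMobility.
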(fn `UserConstructionScript`
  (bind _use_plant (`self.Use Plant`))
  (bind _hierarchicalinstancedstaticmesh3 (`self.HierarchicalInstancedStaticMesh3`))
  (`|ExecutionSequence`
    (:`then_0`
      (`SceneComponent.SetMobility` _hierarchicalinstancedstaticmesh3 (select `bool` _use_plant :`false` "Movable" :`true` "Static" :!type "EComponentMobility Enum"))
      (`SceneComponent.SetMobility` (`self.HierarchicalInstancedStaticMesh4`) (select `bool` _use_plant :`false` "Movable" :`true` "Static" :!type "EComponentMobility Enum"))
      (`SceneComponent.SetMobility` (`self.HierarchicalInstancedStaticMesh2`) (select `bool` _use_plant :`false` "Movable" :`true` "Static" :!type "EComponentMobility Enum"))
      (`SceneComponent.SetMobility` (`self.HierarchicalInstancedStaticMesh1`) (select `bool` _use_plant :`false` "Movable" :`true` "Static" :!type "EComponentMobility Enum"))
      (`SceneComponent.SetVisibility` _hierarchicalinstancedstaticmesh3 _use_plant false)
      (`SceneComponent.SetVisibility` (`self.HierarchicalInstancedStaticMesh4`) _use_plant false)
      (`SceneComponent.SetVisibility` (`self.HierarchicalInstancedStaticMesh2`) _use_plant false)
      (`SceneComponent.SetVisibility` (`self.HierarchicalInstancedStaticMesh1`) _use_plant false))
    (:`then_1`
      (`TextRenderComponent.K2_SetText` (`self.TextRender1`) (`self.Type`))
      (`TextRenderComponent.K2_SetText` (`self.TextRender`) (`self.Type`))
      (if (or (< (.x (`self.GetActorScale3D`)) 0.0) (< (.y (`self.GetActorScale3D`)) 0.0) (< (.z (`self.GetActorScale3D`)) 0.0))
        (`SceneComponent.K2_SetRelativeRotation` (`self.TextRender1`) (struct :`Yaw` 270.0) false false)))
    (:`then_2`
      (for _array_element (`SceneComponent.GetChildrenComponents` (`self.SharedRoot`) false)
        (bind _asstatic_mesh_component (cast `StaticMeshComponent` _array_element))
        (`SceneComponent.SetMobility` _asstatic_mesh_component (`self.Plant Mobility`))))))