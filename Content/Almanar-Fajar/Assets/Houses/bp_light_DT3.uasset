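; Light prop Blueprint from the house assets, with construction-time handling for mirrored placement.
; If any axis of the actor's scale is negative, the construction script adds a 180-degree relative rotation to each direct child of SharedRoot.
; The event graph holds only disabled placeholder events, so the Blueprint adds no runtime logic.
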(fn `UserConstructionScript`
  (bind (_returnvalue_x _returnvalue_y _returnvalue_z) (`KismetMathLibrary.BreakVector` (`self.GetActorScale3D`)))
  (`|ExecutionSequence`
    (:`then_0`
      (if (or (< _returnvalue_x 0.0) (< _returnvalue_y 0.0) (< _returnvalue_z 0.0))
        (for _array_element (`SceneComponent.GetChildrenComponents` (`self.SharedRoot`) false)
          (`SceneComponent.K2_AddRelativeRotation` _array_element (struct :`Pitch` 180.0) false false))))))