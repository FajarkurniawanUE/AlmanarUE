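; House Blueprint for a detached-house asset (vd4, dp4) that displays its Type as text labels.
; The construction script writes Type into two text render components.
; If any axis of the actor's scale is negative, as when mirrored, it sets TextRender1 to a fixed relative rotation.
; The event graph has no active logic, so all behavior runs at construction.
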(fn `UserConstructionScript`
  (`TextRenderComponent.K2_SetText` (`self.TextRender1`) (`self.Type`))
  (`TextRenderComponent.K2_SetText` (`self.TextRender`) (`self.Type`))
  (if (or (< (.x (`self.GetActorScale3D`)) 0.0) (< (.y (`self.GetActorScale3D`)) 0.0) (< (.z (`self.GetActorScale3D`)) 0.0))
    (`SceneComponent.K2_SetRelativeRotation` (`self.TextRender1`) (struct :`Yaw` 270.0) false false)))