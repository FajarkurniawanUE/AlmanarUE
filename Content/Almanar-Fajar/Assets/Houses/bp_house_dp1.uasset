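; House Blueprint for a unit that shows its name and style in a widget when the exterior character traces it.
; Tick compares the character's traced component to Box, toggling input and widget visibility through paired DoOnce gates.
; For other pawns, BeginPlay fills the go-inside widget instead and disables Box collision.
; The construction script toggles instanced plants, labels the type, corrects text rotation for negative scale, and applies mobility to child meshes.
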(event `beingTrace`
  (bind _widget (`self.Widget`))
  (`self.EnableInput` (`GameplayStatics.GetPlayerController` 0))
  (`|ExecutionSequence`
    (:`then_0`
      (`/Engine/EditorBlueprintResources/StandardMacros.DoOnce` false :!label _label
        (:`Completed`
          (`SceneComponent.SetVisibility` _widget true false))))
    (:`then_1`
      (goto _label_2 :!via `Reset`))))

(event `notTrace`
  (`self.DisableInput` (`GameplayStatics.GetPlayerController` 0))
  (`|ExecutionSequence`
    (:`then_0`
      (goto _label :!via `Reset`))
    (:`then_1`
      (`/Engine/EditorBlueprintResources/StandardMacros.DoOnce` false :!label _label_2
        (:`Completed`
          (`SceneComponent.SetVisibility` (`self.Widget`) false false))))))

(event `self.ReceiveTick`
  (params (DeltaSeconds :type "Float (single-precision)"))
  (bind _as_char_roshn_exterior (`self.As Char Roshn Exterior`))
  (`/Engine/EditorBlueprintResources/StandardMacros.IsValid` _as_char_roshn_exterior
    (:`Is Valid`
      (if (== (`/Game/FajarRoshn/Blueprints/char_roshn_exterior.currentTracingComponent` _as_char_roshn_exterior) (`self.Box`))
        (`self.beingTrace`)
        (else
          (`self.notTrace`))))))

(event `self.ReceiveBeginPlay`
  (`SceneComponent.SetVisibility` (`self.Widgetgoinside`) true false)
  (bind _aschar_roshn_exterior (cast `/Game/FajarRoshn/Blueprints/char_roshn_exterior` (`GameplayStatics.GetPlayerCharacter` 0))
    (:`then`
      (set `self.As Char Roshn Exterior` _aschar_roshn_exterior)
      (bind _asumg_unit_info (cast `/Game/FajarRoshn/UMG/umg_unit_info` (`WidgetComponent.GetUserWidgetObject` (`self.Widget`))))
      (set `/Game/FajarRoshn/UMG/umg_unit_info.unit name` (`self.Unit name`) _asumg_unit_info)
      (set `/Game/FajarRoshn/UMG/umg_unit_info.style` (`self.Style`) _asumg_unit_info))
    (:`CastFailed`
      (bind _asumg_goinside_vr_1 (cast `/Game/FajarRoshn/UMG/umg_goinside_vr1` (`WidgetComponent.GetUserWidgetObject` (`self.Widgetgoinside`))))
      (set `/Game/FajarRoshn/UMG/umg_goinside_vr1.unit name` (`self.Unit name`) _asumg_goinside_vr_1)
      (set `/Game/FajarRoshn/UMG/umg_goinside_vr1.style` (`self.Style`) _asumg_goinside_vr_1)
      (`PrimitiveComponent.SetCollisionEnabled` (`self.Box`) "NoCollision"))))

(fn `UserConstructionScript`
  (bind _use_plant (`self.Use Plant`))
  (bind _hierarchicalinstancedstaticmesh1 (`self.HierarchicalInstancedStaticMesh1`))
  (`|ExecutionSequence`
    (:`then_0`
      (`SceneComponent.SetMobility` _hierarchicalinstancedstaticmesh1 (select `bool` _use_plant :`false` "Movable" :`true` "Static" :!type "EComponentMobility Enum"))
      (`SceneComponent.SetMobility` (`self.HierarchicalInstancedStaticMesh2`) (select `bool` _use_plant :`false` "Movable" :`true` "Static" :!type "EComponentMobility Enum"))
      (`SceneComponent.SetMobility` (`self.HierarchicalInstancedStaticMesh3`) (select `bool` _use_plant :`false` "Movable" :`true` "Static" :!type "EComponentMobility Enum"))
      (`SceneComponent.SetVisibility` _hierarchicalinstancedstaticmesh1 _use_plant false)
      (`SceneComponent.SetVisibility` (`self.HierarchicalInstancedStaticMesh2`) _use_plant false)
      (`SceneComponent.SetVisibility` (`self.HierarchicalInstancedStaticMesh3`) _use_plant false)
      (`PrimitiveComponent.SetCastShadow` _hierarchicalinstancedstaticmesh1 _use_plant)
      (`PrimitiveComponent.SetCastShadow` (`self.HierarchicalInstancedStaticMesh2`) _use_plant)
      (`PrimitiveComponent.SetCastShadow` (`self.HierarchicalInstancedStaticMesh3`) _use_plant))
    (:`then_1`
      (`TextRenderComponent.K2_SetText` (`self.TextRender1`) (`self.Type`))
      (if (or (< (.x (`self.GetActorScale3D`)) 0.0) (< (.y (`self.GetActorScale3D`)) 0.0) (< (.z (`self.GetActorScale3D`)) 0.0))
        (`SceneComponent.K2_SetRelativeRotation` (`self.TextRender1`) (struct :`Yaw` 270.0) false false)))
    (:`then_2`
      (for _array_element (`SceneComponent.GetChildrenComponents` (`self.SharedRoot`) false)
        (bind _asstatic_mesh_component (cast `StaticMeshComponent` _array_element))
        (`SceneComponent.SetMobility` _asstatic_mesh_component (`self.Mobility`))))))