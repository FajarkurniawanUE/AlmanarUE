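; Background car actor that shows a random animated car skeletal mesh travelling along a spline.
; BeginPlay picks the car and plays a timeline at Speed that moves the mesh along the spline, keeping the rotation from the spline's start.
; Each pick sets the matching animation and switches on both spotlights and a dynamic material's lamp intensity.
; When the timeline finishes, it picks another car without restarting the timeline.
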(event `useLight?`
  (params (Condition :type Boolean))
  (bind _output_get (set `self.use light?` Condition))
  (`SceneComponent.SetVisibility` (`self.SpotLight1`) _output_get false)
  (`SceneComponent.SetVisibility` (`self.SpotLight`) _output_get false)
  (bind _returnvalue (`KismetMaterialLibrary.CreateDynamicMaterialInstance` (`|GetArrayItem` (`self.LightMaterials`) (`self.RandomIndex`))))
  (`MaterialInstanceDynamic.SetScalarParameterValue` _returnvalue "lampIntensity" (`KismetMathLibrary.SelectFloat` 1.0 0.0 _output_get))
  (`PrimitiveComponent.SetMaterial` (`self.SkeletalMesh`) 0 _returnvalue))

(event `setRandomCar`
  (bind _animtoplay (break `SingleAnimationPlayData` (`|GetArrayItem` (`self.Animation Data`) (`self.RandomIndex`))))
  (bind _output_get (set `self.RandomIndex` (`KismetMathLibrary.RandomIntegerInRange` 0 (`KismetArrayLibrary.Array_LastIndex` (`self.CarSkeletalMesh`)))))
  (`self.useLight?` true)
  (`SkinnedMeshComponent.SetSkinnedAssetAndUpdate` (`self.SkeletalMesh`) (`|GetArrayItem` (`self.CarSkeletalMesh`) (`self.RandomIndex`)) false)
  (set `SkeletalMeshComponent.AnimationData` (make `SingleAnimationPlayData` _animtoplay true true 0.0 (`self.speed`)) (`self.SkeletalMesh`))
  (`SkeletalMeshComponent.SetAnimation` (`self.SkeletalMesh`) _animtoplay)
  (`SkeletalMeshComponent.Play` (`self.SkeletalMesh`) true)
  (`KismetSystemLibrary.PrintString` (`KismetStringLibrary.Conv_IntToString` _output_get)))

(event `self.ReceiveBeginPlay`
  (bind _spline (`self.Spline`))
  (`self.setRandomCar`)
  (`TimelineComponent.SetPlayRate` (`self.Timeline_0`) (`self.speed`))
  (bind (_direction _newtrack_0) (`Timeline|Timeline_0` :!via `PlayFromStart`)
    (:`Update`
      (`SceneComponent.K2_SetWorldTransform` (`self.SkeletalMesh`) (`KismetMathLibrary.MakeTransform` (`SplineComponent.GetLocationAtDistanceAlongSpline` _spline (* (`SplineComponent.GetSplineLength` _spline) _newtrack_0) "World") (`SplineComponent.GetRotationAtDistanceAlongSpline` _spline 0.0 "World")) false false))
    (:`Finished`
      (`self.setRandomCar`))))

(fn `UserConstructionScript`
  (`SceneComponent.SetVisibility` (`self.SpotLight1`) (`self.use light?`) false)
  (`SceneComponent.SetVisibility` (`self.SpotLight`) (`self.use light?`) false))