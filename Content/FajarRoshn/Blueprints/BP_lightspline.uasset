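; BP_lightspline is an actor that places a row of static point lights along a spline.
; The construction script spawns N lights at even distance steps from the spline start, using whole-number spacing from the truncated length.
; Each light takes the shared lumen intensity, attenuation radius and color temperature variables, with reduced indirect lighting intensity.
; The event graph is empty, so it has no runtime logic.
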(fn `UserConstructionScript`
  (for _index (range (`self.N`))
    (bind _returnvalue (`AddComponent|NODE_AddPointLightComponent-0` :`RelativeTransform` (`SplineComponent.GetTransformAtDistanceAlongSpline` (`self.Spline`) (`KismetMathLibrary.Conv_IntToDouble` (* _index (/ (`KismetMathLibrary.FTrunc` (`SplineComponent.GetSplineLength` (`self.Spline`))) (- (`self.N`) 1)))) "Local" false)))
    (`SceneComponent.SetMobility` _returnvalue "Static")
    (`LightComponent.SetIntensity` _returnvalue (`self.Intensity`))
    (`LocalLightComponent.SetIntensityUnits` _returnvalue "Lumens")
    (`LocalLightComponent.SetAttenuationRadius` _returnvalue (`self.Radius`))
    (`LightComponent.SetTemperature` _returnvalue (`self.Temperature`))
    (`LightComponent.SetUseTemperature` _returnvalue true)
    (`LightComponent.SetIndirectLightingIntensity` _returnvalue 0.4)))