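; VR stairs actor that teleports player character 0 between two billboard markers at either end.
; On BeginPlay it hands each of its two umg_stairs_vr widgets a self reference and an Up flag.
; Its teleport event snaps the player to a billboard's location and rotation without sweep, choosing BillboardDown when Up is true and BillboardUp otherwise.
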(event `teleport`
  (params (up :type Boolean))
  (`self.K2_SetActorLocation` (`GameplayStatics.GetPlayerCharacter` 0) (`SceneComponent.K2_GetComponentLocation` (select `bool` up :`false` (`self.Billboard_up`) :`true` (`self.Billboard_down`) :!type "SceneComponent Object Reference")) false false)
  (`self.K2_SetActorRotation` (`GameplayStatics.GetPlayerCharacter` 0) (`SceneComponent.K2_GetComponentRotation` (select `bool` up :`false` (`self.Billboard_up`) :`true` (`self.Billboard_down`) :!type "SceneComponent Object Reference")) false))

(event `self.ReceiveBeginPlay`
  (bind _asumg_stairs_vr (cast `/Game/FajarRoshn/UMG/umg_stairs_vr` (`WidgetComponent.GetUserWidgetObject` (`self.Widgetdown`))))
  (set `/Game/FajarRoshn/UMG/umg_stairs_vr.up` false _asumg_stairs_vr)
  (set `/Game/FajarRoshn/UMG/umg_stairs_vr.bp_stairs_vr` self _asumg_stairs_vr)
  (bind _asumg_stairs_vr_2 (cast `/Game/FajarRoshn/UMG/umg_stairs_vr` (`WidgetComponent.GetUserWidgetObject` (`self.Widgetup`))))
  (set `/Game/FajarRoshn/UMG/umg_stairs_vr.up` true _asumg_stairs_vr_2)
  (set `/Game/FajarRoshn/UMG/umg_stairs_vr.bp_stairs_vr` self _asumg_stairs_vr_2))

(fn `UserConstructionScript`)