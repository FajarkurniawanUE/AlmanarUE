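; Curb spline actor that builds a row of spline meshes along its spline in the Construction Script, with no active gameplay logic.
; It divides spline length by MeshLength and adds one segment per whole step, each using an unseeded random pick from Meshes scaled by Width and Height.
; Tangents are clamped to MeshLength so each segment follows the curve.
; An unconnected per-spline-point cable builder remains in the graph and never runs.
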(fn `UserConstructionScript`
  (bind _spline (`self.Spline`))
  (bind _spline_2 (`self.Spline`))
  (bind _meshes (`self.Meshes`))
  (bind _returnvalue (`KismetMathLibrary.MakeVector2D` (`self.Width`) (`self.Height`)))
  (bind _returnvalue_2 (`KismetMathLibrary.FTrunc` (/ (`SplineComponent.GetSplineLength` (`self.Spline`)) (`self.MeshLength`))))
  (if (> _returnvalue_2 0)
    (for _index (range _returnvalue_2)
      (bind _returnvalue_3 (`AddComponent|NODE_AddSplineMeshComponent-1`))
      (`StaticMeshComponent.SetStaticMesh` _returnvalue_3 (`|GetArrayItem` _meshes (`KismetMathLibrary.RandomIntegerInRange` 0 (`KismetArrayLibrary.Array_LastIndex` _meshes))))
      (`SplineMeshComponent.SetStartScale` _returnvalue_3 _returnvalue true)
      (`SplineMeshComponent.SetEndScale` _returnvalue_3 _returnvalue true)
      (bind _returnvalue_4 (* _index (`self.MeshLength`)))
      (bind _returnvalue_5 (* (+ _index 1) (`self.MeshLength`)))
      (`SplineMeshComponent.SetStartAndEnd` _returnvalue_3 (`SplineComponent.GetLocationAtDistanceAlongSpline` _spline_2 _returnvalue_4 "Local") (`KismetMathLibrary.ClampVectorSize` (`SplineComponent.GetTangentAtDistanceAlongSpline` _spline_2 _returnvalue_4 "Local") 0.0 (`self.MeshLength`)) (`SplineComponent.GetLocationAtDistanceAlongSpline` _spline _returnvalue_5 "Local") (`KismetMathLibrary.ClampVectorSize` (`SplineComponent.GetTangentAtDistanceAlongSpline` _spline _returnvalue_5 "Local") 0.0 (`self.MeshLength`)) true)
      (`SceneComponent.K2_AttachToComponent` _returnvalue_3 (`self.Spline`) "None" "KeepRelative" "KeepRelative" "KeepRelative" true))))