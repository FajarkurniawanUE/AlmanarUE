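; Actor that toggles a referenced planar reflection according to whether its mirror mesh is on screen, so the reflection is hidden when unseen.
; The reflection starts hidden and stays hidden while the player pawn is pawn_dollhouse.
; Otherwise Tick checks WasRecentlyRendered on the mirror, and two cross-reset DoOnce gates set visibility only when that state changes.
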(event `self.ReceiveBeginPlay`
  (`SceneComponent.SetVisibility` (`PlanarReflection.PlanarReflectionComponent` (`self.planar`)) false false))

(event `self.ReceiveTick`
  (params (DeltaSeconds :type "Float (single-precision)"))
  (bind _rootcomponent (`Actor.RootComponent` (`self.planar`)))
  (cast `/Game/FajarRoshn/Blueprints/pawn_dollhouse` (`GameplayStatics.GetPlayerPawn` 0)
    (:`then`
      (`SceneComponent.SetVisibility` (`PlanarReflection.PlanarReflectionComponent` (`self.planar`)) false false))
    (:`CastFailed`
      (cast `/Game/FajarRoshn/Blueprints/char_roshn` (`GameplayStatics.GetPlayerCharacter` 0)
        (:`then`
          _)
        (:`CastFailed`
          _))
      (if (`self.WasRecentlyRendered` (`self.MirrorStaticMesh`) 0.2)
        (`|ExecutionSequence`
          (:`then_0`
            (`/Engine/EditorBlueprintResources/StandardMacros.DoOnce` false :!label _label
              (:`Completed`
                (`SceneComponent.SetVisibility` _rootcomponent true false))))
          (:`then_1`
            (goto _label_2 :!via `Reset`)))
        (else
          (`|ExecutionSequence`
            (:`then_0`
              (goto _label :!via `Reset`))
            (:`then_1`
              (`/Engine/EditorBlueprintResources/StandardMacros.DoOnce` false :!label _label_2
                (:`Completed`
                  (`SceneComponent.SetVisibility` _rootcomponent false false))))))))))

(fn `UserConstructionScript`)