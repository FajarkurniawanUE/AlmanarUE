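; Car prop Blueprint, apparently a Lucid Air by its name, with configurable paint and a fake shadow plane.
; The Construction Script builds a dynamic paint material using the custom Color or a random pick from four presets, re-rolled on each construction, for three body meshes.
; It also sets the shadow plane's opacity and applies RoofMobility to StaticMesh.
; The Event Graph is inactive, and leftover material and mobility logic is disconnected.
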(event `self.ReceiveBeginPlay`)

(fn `UserConstructionScript`
  (`|ExecutionSequence`
    (:`then_1`
      (`|ExecutionSequence`
        (:`then_0`
          (bind _returnvalue (`KismetMaterialLibrary.CreateDynamicMaterialInstance` "/Game/Almanar-Fajar/Materials/MI_carpaint_Inst.MI_carpaint_Inst"))
          (set `self.NewVar_1` _returnvalue)
          (`MaterialInstanceDynamic.SetVectorParameterValue` (`self.NewVar_1`) "BaseColor" (`KismetMathLibrary.SelectColor` (`self.Color`) (select `int` (`KismetMathLibrary.RandomIntegerInRange` 0 3) :`0` (struct :`R` 0.508762 :`G` 0.578107 :`B` 0.630208 :`A` 1.0) :`1` (struct :`R` 0.182292 :`G` 0.182292 :`B` 0.182292 :`A` 1.0) :`2` (struct :`R` 0.331597 :`G` 0.041392 :`B` 0.04689 :`A` 1.0) :`3` (struct :`R` 0.04889 :`G` 0.129676 :`B` 0.331597 :`A` 1.0) :!type "LinearColor Structure") (`self.Custom Color`)))
          (`PrimitiveComponent.SetMaterial` (`self.Object002_StaticMeshComponent0`) 0 (`self.NewVar_1`))
          (`PrimitiveComponent.SetMaterial` (`self.Object003_StaticMeshComponent0`) 0 (`self.NewVar_1`))
          (`PrimitiveComponent.SetMaterial` (`self.Object001_StaticMeshComponent0`) 0 (`self.NewVar_1`)))
        (:`then_1`
          (bind _returnvalue_2 (`KismetMaterialLibrary.CreateDynamicMaterialInstance` "/Game/Almanar-Fajar/Materials/MI_layer_shadow.MI_layer_shadow"))
          (set `self.NewVar_0` _returnvalue_2)
          (`MaterialInstanceDynamic.SetScalarParameterValue` (`self.NewVar_0`) "Opacity" (`self.Shadow Strenght`))
          (`PrimitiveComponent.SetMaterial` (`self.Plane`) 0 (`self.NewVar_0`)))
        (:`then_2`
          (`SceneComponent.SetMobility` (`self.StaticMesh`) (`self.Roof Mobility`)))))))