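; Lucid Air car prop Blueprint with an adjustable body color and shadow strength.
; The construction script applies a dynamic car paint material tinted by Color to four body meshes, and a second dynamic material with ShadowStrenght as opacity to a Plane.
; BeginPlay and Tick do nothing; an event-graph copy of the material setup and a mobility-based shadow-casting toggle are left unconnected.
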(event `self.ReceiveBeginPlay`)

(fn `UserConstructionScript`
  (bind _returnvalue (`KismetMaterialLibrary.CreateDynamicMaterialInstance` "/Game/Almanar-Fajar/Materials/MI_carpaint_Inst.MI_carpaint_Inst"))
  (set `self.NewVar_1` _returnvalue)
  (`MaterialInstanceDynamic.SetVectorParameterValue` (`self.NewVar_1`) "BaseColor" (`self.Color`))
  (`PrimitiveComponent.SetMaterial` (`self.Object002_StaticMeshComponent0`) 0 (`self.NewVar_1`))
  (`PrimitiveComponent.SetMaterial` (`self.Object003_StaticMeshComponent0`) 0 (`self.NewVar_1`))
  (`PrimitiveComponent.SetMaterial` (`self.Object001_StaticMeshComponent0`) 0 (`self.NewVar_1`))
  (`PrimitiveComponent.SetMaterial` (`self.Object005_StaticMeshComponent0`) 0 (`self.NewVar_1`))
  (bind _returnvalue_2 (`KismetMaterialLibrary.CreateDynamicMaterialInstance` null))
  (set `self.NewVar_0` _returnvalue_2)
  (`MaterialInstanceDynamic.SetScalarParameterValue` (`self.NewVar_0`) "Opacity" (`self.Shadow Strenght`))
  (`PrimitiveComponent.SetMaterial` (`self.Plane`) 0 (`self.NewVar_0`)))